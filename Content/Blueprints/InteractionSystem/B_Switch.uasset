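; B_Switch is an interactable switch that toggles a target light off and on.
; It caches the light's intensity at BeginPlay, then each Interact flips the Switched state and sets intensity to zero or back to the cached value.
; A timeline simultaneously rolls the Button component toward a positive or negative target angle and prints a debug string when finished.
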(event Custom|TurnLight
  (params (On%20/%20Off :type Boolean))
  (bind _targetlight (Variables|Default|GetTargetLight))
  (bind _lightcomponent (Variables|/Script/Engine.Light|GetLightComponent _targetlight))
  (if On%20/%20Off
    (Rendering|Components|Light|SetIntensity _lightcomponent (Variables|Default|GetIntensity))
    (else
      (Rendering|Components|Light|SetIntensity _lightcomponent 0.0))))

(event EventInteract
  (params (Player%20Controller :type Player%20Controller%20Object%20Reference))
  (if (not (Variables|Default|GetSwitched))
    (Variables|Default|SetSwitched true)
    (CallFunction|TurnLight false)
    (Variables|Default|SetTargetRotation 1e+01)
    (bind _alpha (Timeline|Timeline PlayFromStart)
      (:Update
        (Transformation|SetRelativeRotation (Variables|Default|Getbutton) (Math|Rotator|MakeRotator (* _alpha (Variables|Default|GetTargetRotation)) 0.0 0.0) false false))
      (:Finished
        (Development|PrintString "switched")))
    (else
      (Variables|Default|SetSwitched false)
      (CallFunction|TurnLight true)
      (Variables|Default|SetTargetRotation -1e+01)
      (Timeline|Timeline PlayFromStart))))

(event EventBeginPlay
  (Variables|Default|SetIntensity (Variables|/Script/Engine.LightComponentBase|GetIntensity (Variables|/Script/Engine.Light|GetLightComponent (Variables|Default|GetTargetLight)))))

(fn ConstructionScript)