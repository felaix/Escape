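; Cable puzzle plug that the player can pick up and drag in front of the camera.
; Interact starts the drag only if the plug is Movable and not already moved; this file never clears that flag.
; A fast looping timer sweeps the actor to a point lerped between its location and a spot ahead of the camera.
; DropItem pauses that timer to stop the movement.
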(event Custom|OnUpdate
  (Transformation|SetActorLocation (.Lerp (|GetCamera 0.2)) true true))

(event Custom|DropItem
  (Utilities|Time|PauseTimerbyHandle (Variables|Default|GetTimer)))

(event Custom|DragItem
  (bind _returnvalue (Utilities|Time|SetTimerbyEvent (delegate Custom|OnUpdate) 0.01 true))
  (Variables|Default|SetTimer _returnvalue))

(event EventInteract
  (params (Player%20Controller :type Player%20Controller%20Object%20Reference))
  (if (not (Variables|Default|GetAlready%20Moved))
    (if (Variables|Default|GetMovable?)
      (CallFunction|DragItem)
      (Variables|Default|SetAlready%20Moved true))))

(event EventBeginPlay
  (Variables|Default|SetCharRef (Game|GetPlayerCharacter 0))
  (Variables|Default|SetPlayerCtrlRef (Game|GetPlayerController 0)))

(fn ConstructionScript)