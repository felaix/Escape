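; Player interaction component that finds interactable objects in view, triggers interaction and inspection, and doubles as the flashlight toggle.
; A looping timer capsule-traces from the player camera and caches the hit actor only if it implements I_Interactable.
; Interact messages that actor and broadcasts OnInspectObject, or toggles the character's spotlight when there is no target.
; RotateInspectable applies local rotation to the cached actor for inspection.
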(event Custom|OnUpdate
  (bind _characterref (Variables|Essential|GetCharacterRef))
  (bind _outhit (Class|KismetSystemLibrary|CapsuleTraceSingleforObjects (CallFunction|GetCameraLocation _characterref) (CallFunction|GetCameraDistanceLocation _characterref (Variables|Default|GetDistance)) 25.0 25.0 (Variables|Config|GetInteractableObjectType) false (Utilities|Array|MakeArray (Variables|Essential|GetCharacterRef)) "None" true "(R=1.000000,G=0.000000,B=0.000000,A=1.000000)" "(R=0.000000,G=1.000000,B=0.000000,A=1.000000)" 1.0))
  (if (.bBlockingHit (Collision|BreakHitResult _outhit))
    (if (Utilities|DoesObjectImplementInterface (.HitActor (Collision|BreakHitResult _outhit)) "/Game/Blueprints/InteractionSystem/I_Interactable.I_Interactable_C")
      (Variables|Essential|SetInteractableActor (.HitActor (Collision|BreakHitResult _outhit)))
      (else
        (Variables|Essential|SetInteractableActor 0 :!label _label)))
    (else
      (goto _label))))

(event Custom|Interact
  (bind _interactableactor (Variables|Essential|GetInteractableActor))
  (bind _flashlight (Variables|Default|GetFlashlight))
  (Utilities|IsValid _interactableactor
    (:Is%20Valid
      (Class|IInteractable|Interact(Message) _interactableactor)
      (Default|CallOnInspectObject _interactableactor))
    (:Is%20Not%20Valid
      (Development|PrintString "flashlight on/off")
      (Rendering|SetVisibility _flashlight (not (Rendering|IsVisible _flashlight)) false))))

(event Custom|RotateInspectable
  (params (Rotation :type Rotator))
  (bind _interactableactor (Variables|Essential|GetInteractableActor)
    (:then
      (Transformation|AddActorLocalRotation _interactableactor Rotation false false))
    (:else
      (Development|PrintString "Not valid"))))

(event EventBeginPlay
  (bind _output_get (Variables|Essential|SetCharacterRef (Game|GetPlayerCharacter 0)))
  (Variables|Default|SetFlashlight (Actor|GetComponentbyClass _output_get "/Script/Engine.SpotLightComponent"))
  (Utilities|Time|SetTimerbyEvent (delegate Custom|OnUpdate) 0.1 true))