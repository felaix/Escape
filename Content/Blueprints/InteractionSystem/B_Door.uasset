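; Interactable door Blueprint that swings 90 degrees in a direction chosen by whether something overlaps its front box.
; Interact calls Open or Close based on IsOpen, which is never set in these graphs.
; A Timeline lerps the Scene component's relative rotation and plays in reverse to close.
; Leaving FrontBox clears InFront and closes the door; GetCameraPos just returns a zero vector.
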(event OnComponentBeginOverlap(FrontBox)
  (params (OverlappedComponent :type Primitive%20Component%20Object%20Reference) (OtherActor :type Actor%20Object%20Reference) (OtherComp :type Primitive%20Component%20Object%20Reference) (OtherBodyIndex :type Integer) (bFromSweep :type Boolean) (SweepResult :type Hit%20Result%20Structure%20%28by%20ref%29))
  (Variables|Default|SetinFront true))

(event OnComponentEndOverlap(FrontBox)
  (params (OverlappedComponent :type Primitive%20Component%20Object%20Reference) (OtherActor :type Actor%20Object%20Reference) (OtherComp :type Primitive%20Component%20Object%20Reference) (OtherBodyIndex :type Integer))
  (Variables|Default|SetinFront false)
  (CallFunction|Close))

(event Custom|Open
  (bind _alpha (Timeline|Timeline PlayFromStart)
    (:Update
      (Transformation|SetRelativeRotation (Variables|Default|GetScene) (Math|Rotator|Lerp(Rotator) "0,0.000000, 0" (select (Variables|Default|GetinFront) "0,90.000000, 0" "0,-90.000000, 0") _alpha true) false false))))

(event Custom|Close
  (bind _alpha (Timeline|Timeline Reverse)
    (:Update
      (Transformation|SetRelativeRotation (Variables|Default|GetScene) (Math|Rotator|Lerp(Rotator) "0,0.000000, 0" (select (Variables|Default|GetinFront) "0,90.000000, 0" "0,-90.000000, 0") _alpha true) false false))))

(event EventInteract
  (if (Variables|Default|GetisOpen)
    (CallFunction|Close)
    (else
      (CallFunction|Open))))

(fn ConstructionScript)

(fn GetCameraPos
  (return "0, 0, 0"))