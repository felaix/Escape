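; B_Inventory is an inventory Blueprint that stores item IDs and keeps an on-screen widget in step with them.
; On BeginPlay it creates a W_Inventory widget and adds it to the viewport.
; Add and remove functions update the Inventory collection and then call the widget, though the removal display call receives no item ID.
; A check function reports whether a given ID is held.
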(event EventBeginPlay
  (bind _returnvalue (UserInterface|CreateWidget "/Game/Blueprints/InventorySystem/TexturesAndWidgets/Inventory/W_Inventory.W_Inventory_C"))
  (UserInterface|Viewport|AddtoViewport _returnvalue 0)
  (Variables|Default|SetInventory%20Widget _returnvalue))

(fn ConstructionScript)

(fn AddItemtoInventory
  (params (Item%20ID :type String))
  (Utilities|Array|Add (Variables|Default|GetInventory) Item%20ID)
  (Default|DisplayInventoryItem (Variables|Default|GetInventory%20Widget) Item%20ID))

(fn RemoveItemfromInventory
  (params (Item%20ID :type String))
  (Utilities|Array|RemoveItem (Variables|Default|GetInventory) Item%20ID)
  (Default|RemoveInventoryItemDisplay (Variables|Default|GetInventory%20Widget)))

(fn CheckforItem
  (params (Item%20ID :type String))
  (return (Utilities|Array|ContainsItem (Variables|Default|GetInventory) Item%20ID)))