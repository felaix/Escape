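; Blueprint function library that limits how far the player can rotate the camera view.
; Set Player Camera View writes caller-supplied pitch and yaw bounds to the player camera manager.
; Reset Player Camera View restores those bounds to hard-coded defaults.
; Both functions always fetch the manager for player index 0, using the passed PlayerController only as world context.
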(fn SetPlayerCameraView
  (params (Min%20Pitch :type Float%20%28double-precision%29) (Max%20Pitch :type Float%20%28double-precision%29) (Min%20Yaw :type Float%20%28double-precision%29) (Max%20Yaw :type Float%20%28double-precision%29) (Player%20Controller :type Player%20Controller%20Object%20Reference))
  (bind _returnvalue (Game|GetPlayerCameraManager Player%20Controller))
  (Variables|/Script/Engine.PlayerCameraManager|SetViewPitchMin _returnvalue Min%20Pitch)
  (Variables|/Script/Engine.PlayerCameraManager|SetViewPitchMax _returnvalue Max%20Pitch)
  (Variables|/Script/Engine.PlayerCameraManager|SetViewYawMin _returnvalue Min%20Yaw)
  (Variables|/Script/Engine.PlayerCameraManager|SetViewYawMax _returnvalue Max%20Yaw))

(fn ResetPlayerCameraView
  (params (Player%20Controller :type Player%20Controller%20Object%20Reference))
  (bind _returnvalue (Game|GetPlayerCameraManager Player%20Controller))
  (Variables|/Script/Engine.PlayerCameraManager|SetViewPitchMin _returnvalue -45.0)
  (Variables|/Script/Engine.PlayerCameraManager|SetViewPitchMax _returnvalue 45.0)
  (Variables|/Script/Engine.PlayerCameraManager|SetViewYawMin _returnvalue -179.0)
  (Variables|/Script/Engine.PlayerCameraManager|SetViewYawMax _returnvalue 179.0))