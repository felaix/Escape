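; First-person player controller that routes move, look, jump and interact input to the C_Character pawn and the interaction system component.
; A SwitchControllerState macro gates axis input: Movement walks and looks, while Inspect rotates the inspected object.
; SetState stores the previous state and toggles character movement, binding empty inspect/uninspect handlers.
; Jump and Interact ignore state; Grab, Keypad and Laser states exist but are unhandled here.
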(event Custom|Switch%20on%20State
  (bind _fpref (Variables|Default|GetFPRef))
  (bind _ac_interactionsystem (Variables|Default|GetAC_InteractionSystem))
  (bind _charactermovement (Variables|/Script/Engine.Character|GetCharacterMovement _fpref))
  ;[0 0 0] Enable / Disable Movement on State [Inspect] and [Movement]
  (Utilities|SwitchControllerState
    (:Movement
      (Components|Activation|Activate _charactermovement true)
      (EventDispatchers|BindEventtoOnUninspectObject _ac_interactionsystem (delegate Custom|OnUnInspect)))
    (:Inspect
      (Components|Activation|Deactivate _charactermovement)
      (EventDispatchers|BindEventtoOnInspectObject _ac_interactionsystem (delegate Custom|OnInspect)))))

(event Custom|OnInspect
  (params (Inspect%20Object :type Actor%20Object%20Reference))
  ;[0 0 0] Enable / Disable Movement on State [Inspect] and [Movement]
)

(event Custom|OnUnInspect
  ;[0 0 0] Enable / Disable Movement on State [Inspect] and [Movement]
)

(event EventBeginPlay
  ;[0 0 0] Start
  (bind _asc_character (Utilities|Casting|CastToC_Character (Game|GetPlayerCharacter 0)))
  (Variables|Default|SetFPRef _asc_character))

(event EventSetState
  (params (State :type E_PlayerState%20Enum :default "NewEnumerator0"))
  ;[0 0 0] Set State
  (Variables|Default|SetPrevState (Variables|Default|GetCurState))
  (Variables|Default|SetCurState State)
  (CallFunction|SwitchonState))

(event Input|ActionEvents|InputActionJump
  (params (Key :type Key%20Structure :default "None"))
  ;[0 0 0] Inputs
  (:Pressed
    (Default|DoJump (Variables|Default|GetFPRef))))

(event Input|ActionEvents|InputActionInteract
  (params (Key :type Key%20Structure :default "None"))
  ;[0 0 0] Inputs
  (:Pressed
    (Default|Interact (Variables|Default|GetAC_InteractionSystem))))

(event Input|AxisEvents|InputAxisMoveForwardBackward
  (params (AxisValue :type Float%20%28single-precision%29))
  ;[0 0 0] Inputs
  (bind _output_get (Variables|InputValues|SetForwardBackwardValue AxisValue))
  (Utilities|SwitchControllerState
    (:Movement
      (Default|MoveForwardBackward (Variables|Default|GetFPRef) _output_get))))

(event Input|AxisEvents|InputAxisMoveLeftRight
  (params (AxisValue :type Float%20%28single-precision%29))
  ;[0 0 0] Inputs
  (bind _output_get (Variables|InputValues|SetLeftRightValue AxisValue))
  (Utilities|SwitchControllerState
    (:Movement
      (Default|MoveLeftRight (Variables|Default|GetFPRef) _output_get))))

(event Input|AxisEvents|InputAxisLookLeftRight
  (params (AxisValue :type Float%20%28single-precision%29))
  ;[0 0 0] Inputs
  (bind _output_get (Variables|InputValues|SetYaw AxisValue))
  (Utilities|SwitchControllerState
    (:Movement
      (Pawn|Input|AddControllerYawInput (Variables|Default|GetFPRef) _output_get))
    (:Inspect
      (Default|RotateInspectable (Variables|Default|GetAC_InteractionSystem) (Math|Rotator|MakeRotator 0.0 0.0 _output_get)))))

(event Input|AxisEvents|InputAxisLookUpDown
  (params (AxisValue :type Float%20%28single-precision%29))
  ;[0 0 0] Inputs
  (bind _output_get (Variables|InputValues|SetPitch AxisValue))
  (Utilities|SwitchControllerState
    (:Movement
      (Pawn|Input|AddControllerPitchInput (Variables|Default|GetFPRef) _output_get))
    (:Inspect
      (Default|RotateInspectable (Variables|Default|GetAC_InteractionSystem) (Math|Rotator|MakeRotator 0.0 _output_get 0.0)))))

(fn ConstructionScript)